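; Shotgun enemy NPC that fires a three-bullet spread toward the player and reports its death to an enemy spawner.
; A looping FireWeapon timer, started and stopped by StartFiring and StopFiring, spawns yaw-rotated projectiles while both characters are alive.
; TakeDamage reduces health; at zero or below, with a valid spawner, it updates the spawner's counts, launches the physics-simulated mesh along the hit impulse and destroys the actor after a delay.
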(event Custom|StartFiring
  (Utilities|Time|SetTimerbyFunctionName 0 "FireWeapon" (Variables|Default|GetFireRate) true))

(event Custom|FireWeapon
  (Variables|Default|SetIsShooting true)
  (bind _isdead (Default|GetIsDead (.AsTop%20Down%20Character (Utilities|Casting|CastToTopDownCharacter (Game|Player|GetPlayerPawn 0)))))
  (if (not _isdead)
    (if (not (Variables|Default|GetDead))
      (if (Utilities|IsValid (Game|Player|GetPlayerPawn 0))
        (CallFunction|SpawnBullet 0.0)
        (CallFunction|SpawnBullet -45.0)
        (CallFunction|SpawnBullet 45.0)
        (else
          (Variables|Default|SetIsShooting true)))
      (else
        (Variables|Default|SetIsShooting false)))
    (else
      (Variables|Default|SetIsShooting false))))

(event Custom|StopFiring
  (Utilities|Time|ClearTimerbyFunctionName 0 "FireWeapon")
  (Variables|Default|SetIsShooting false))

(event Custom|DestroySelf
  (Actor|DestroyActor))

(event Collision|EventActorBeginOverlap
  (params (OtherActor :type Actor%20Object%20Reference)))

(event EventTick
  (params (DeltaSeconds :type Float%20%28single-precision%29)))

(event EventTakeDamage
  (params (i_Damage :type Integer) (Impulse :type Vector :default "0, 0, 0"))
  (bind _enemyspawner (Variables|Default|GetEnemySpawner))
  ;[1 1 1] Take Damage & Check for Death
  (Variables|Default|SetImpulseDirection Impulse)
  (bind _output_get (Variables|Default|SetHealth (- (Variables|Default|GetHealth) i_Damage)))
  (Math|Integer|CompareInt _output_get
    (:==
      _)
    (:<
      _))
  (Variables|Default|SetDead true)
  (if (Utilities|IsValid _enemyspawner)
    (Default|DecrementSpawnCountIncrementKill _enemyspawner)
    (Collision|SetCollisionEnabled (Variables|Collision|GetCapsuleComponent) "NoCollision")
    (Physics|SetSimulatePhysics (Variables|Character|GetMesh) true)
    (Physics|AddImpulse (Variables|Character|GetMesh) (* (Math|Vector|MakeVector (.x (Variables|Default|GetImpulseDirection)) (.y (Variables|Default|GetImpulseDirection)) (+ (.z (Variables|Default|GetImpulseDirection)) 3e+02)) (Variables|Default|GetFlyAwayStrength)) "None" false)
    (Utilities|Time|SetTimerbyFunctionName 0 "DestroySelf" 2.0)))

(fn ConstructionScript)

(fn SetEnemySpawner
  (params (EnemySpawner :type Enemy%20Spawner%20Object%20Reference))
  (Variables|Default|SetEnemySpawner EnemySpawner))

(fn SpawnBullet
  (params (RotateAmount :type Float%20%28single-precision%29))
  (bind _returnvalue (Game|SpawnActorfromClass "/Game/_Gameplay/BulletShotgun.BulletShotgun_C" (Math|Transform|MakeTransform (Transformation|GetWorldLocation (Variables|Default|GetFireLocation)) "0, 0, 0" "0.050000,0.050000,0.050000") "Undefined" 0 0))
  (if (Utilities|IsValid _returnvalue)
    (Default|SetVelocity _returnvalue (* (Math|Vector|RotateVector (Math|Vector|GetUnitDirection(Vector) (Transformation|GetActorLocation) (Transformation|GetActorLocation (Game|Player|GetPlayerPawn 0))) (Math|Rotator|MakeRotator 0.0 0.0 RotateAmount)) 4e+02))))

(fn GetPoints
  (return (Variables|Default|GetPoints)))